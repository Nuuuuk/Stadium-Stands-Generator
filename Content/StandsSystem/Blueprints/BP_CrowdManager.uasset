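; Crowd manager for the stands system that bakes spectators as HISM instances of human static meshes with VAT (vertex animation texture) materials.
; The construction script links the first GlobalSeatManager found if none is set, then calls the parent script for the first-spawn bake.
; AutoBakeSlow optionally rebakes on each construction run.
; HISMsRoot gets the inverse actor transform as its relative transform, cancelling the actor's placement.
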(fn `UserConstructionScript`
  (`|ExecutionSequence`
    (:`then_0`
      ;[0 0 0 0.75] Auto Hookup SeatManager
      (`/Engine/EditorBlueprintResources/StandardMacros.IsValid` (`self.SeatManager`)
        (:`Is Valid`)
        (:`Is Not Valid`
          (bind _outactors (`GameplayStatics.GetAllActorsOfClass` "/Script/Stadium56.AGlobalSeatManager"))
          (set `self.SeatManager` (`|GetArrayItem` _outactors)))))
    (:`then_1`
      (`parent.UserConstructionScript`) ; this just bake the crowd at FIRST spawn
    )
    (:`then_2`
      ;[0 0 0 0.75] auto bake?
      (if (`self.autoBake (slow)`)
        (`self.BakeCrowd` :!pinned true) ; 1. Clear the existing HISMs\n\n2. create the HISM components (given the assets set in this bp: the human SMs & their MI_VATs)\n\n3. filter all transforms (from BP_Seat_Manager) by the volumes (from BP_CrowdVolume)\n\n4. Fill HISMs (a random float 0-1 was sent to each instance (for random animation offst))
      ))
    (:`then_3`
      ;[0 0 0 0.75] invert offset the world transform
      (`SceneComponent.K2_SetRelativeTransform` (`self.HISMsRoot`) (`KismetMathLibrary.InvertTransform` (`self.GetTransform`)) false false))))